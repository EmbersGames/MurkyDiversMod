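; Base Blueprint for player gameplay abilities, adding animation-end cancelling and input buffering on top of its parent's setup and finish events.
; When cancelling becomes allowed, it sets a tag, removes lock tags and signals the input buffer to proceed.
; Gameplay events then let the ability's montage stop and the ability end early.
; Motion warping, targeting, interact-actor and client prediction helpers are empty stubs here.
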(event EventSetupAbilityStart
  (|CallParentFunction))

(event EventInitVariables
  (|CallParentFunction))

(event EventFinishAbility
  (|CallParentFunction))

(event EventBindGameplayEvents
  (|CallParentFunction))

(event Custom|Event_CanCancelEndOfAnim
  (if (not (Variables|Default|GetSetCanCancelAnimEnd))
    (Default|CallCanCancelEndOfAnim self)
    (Class|GameplayAbilityBase|SetGameplayTagCount "(TagName=\"Player.Action.System.CanCancelAnimEnd\")" 1)
    (Variables|Default|SetSetCanCancelAnimEnd true)
    (Class|GameplayAbilityBase|RemoveTagstoLockAll)
    (Ability|SendGameplayEvent "(TagName=\"System.BufferInput.Proceed_Event\")")))

(event Custom|CancelMyAnimEnd
  (Animation|Montage|MontageStop -1.0)
  (Ability|EndAbility))

(event Custom|Event_StartBufferInputRecording
  (Class|GameplayAbilityBase|SetGameplayTagCount "(TagName=\"System.BufferInput.IsRecording\")" 1))

(event Custom|SendCancelAnimEnd
  (if (Class|AbilitySystemComponentBase|HasGameplayTag (Class|GameplayAbilityBase|GetOwnerAbilitySystemComponent) "(TagName=\"Player.Action.System.CanCancelAnimEnd\")")
    (Ability|SendGameplayEvent "(TagName=\"Action.CurrentAction.CancelAnimEndEvent\")")
    (Class|AbilitySystemComponentBase|SetGameplayTagCount (Class|GameplayAbilityBase|GetOwnerAbilitySystemComponent) "(TagName=\"Player.Action.System.CanCancelAnimEnd\")" 0)))

(event Custom|BindCancelAnimEndEvent
  (Ability|Tasks|WaitGameplayEvent "(TagName=\"Player.Action.System.CancelAnimEnd_Event\")" 0
    (:EventReceived
      (if (Variables|Default|GetSetCanCancelAnimEnd)
        (CallFunction|CancelMyAnimEnd)))))

(fn NewMontageEventReceive
  (params (Tag :type Gameplay%20Tag%20Structure) (EventData :type Gameplay%20Event%20Data%20Structure))
  (|CallParentFunction Tag EventData))

(fn UpdateMotionWarpingTarget
  (params (MotionWarpingComp :type Motion%20Warping%20Component%20Base%20Object%20Reference) (Notify :type Object%20Object%20Reference) (RootMotionModifier :type Root%20Motion%20Modifier%20Object%20Reference)))

(fn StartMotionWarpingTarget
  (params (MotionWarpingComp :type Motion%20Warping%20Component%20Base%20Object%20Reference) (Notify :type Object%20Object%20Reference) (RootMotionModifier :type Root%20Motion%20Modifier%20Object%20Reference)))

(fn GetPlayerTargetingComp
  (return))

(fn GetLastMotionWarpingTarget
  (params (MaxDistance :type Float%20%28double-precision%29) (MaxAngle :type Float%20%28double-precision%29))
  (return 0))

(fn IsValidMotionWarpingTarget
  (params (Actor :type Actor%20Object%20Reference) (MaxDistance :type Float%20%28double-precision%29))
  (return false))

(fn GetBestInteractActor
  (return 0))

(fn GetBestHeavyInteractActor
  (return 0))

(fn SetClientMovementPrediction
  (params (Enable :type Boolean)))

(fn IsOwningClient
  (return false))