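; Base player ability manager component that declares the interface for granting, looking up and activating Gameplay Abilities on the player; every graph here is an empty stub.
; Its events outline initialization after possession and GAS readiness, with event binding split by server, owning client and other clients.
; Further hooks cover replicated ability grants, buffered input triggers, unlock checks, interact and grab target selection, and client movement prediction.
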(event Custom|GiveAbility)

(event Custom|NewAbilityAdded_Rep
  (params (GameplayAbility :type Gameplay%20Ability%20Object%20Reference)))

(event Custom|BindAbilityEvent_OnOtherClient)

(event Custom|BindGameplayEvent_OnOtherClient)

(event Custom|WaitPossessionForinitialization)

(event Custom|SearchAbilityForClient)

(event Custom|BindGameplayEvent_AllRoles)

(event Custom|Internal_BindGameplayEvent_AllRoles)

(event Custom|Internal_ComponentInitialisationWhenGasReady)

(event Custom|WaitBufferInput_Proceed_Event)

(event Custom|WaitBufferInput_Clear_Event)

(event Custom|TrySaveInBufferInput_TriggerEvent)

(event Custom|BindAbilityEvent_OnServer)

(event Custom|BindGameplayEvent_OnServer)

(event Custom|SetupAMC)

(event Custom|BindGameplayEvent_OnOwningClient)

(event Custom|BindAbilityEvent_OnOwningClient)

(event EventEndPlay
  (params (EndPlayReason :type EEndPlayReason%20Enum :default "Destroyed")))

(event EventComponentInitialization)

(fn HandleNewTrigger
  (params (FromBufferInput :type Boolean))
  (return true))

(fn GetAbilityInstance
  (return))

(fn GetAbilitytoActivate
  (return ""))

(fn GetAbilityInstancetoActivate
  (return 0))

(fn GetInputPlayerSubSystem
  (return 0))

(fn AbilityIsUnlock
  (return false))

(fn OnRepComponentInitialized?)

(fn CheckBestInteractActor
  (params (SimpleInteract :type Boolean) (HeavyGrababable :type Boolean) (Grabable :type Boolean))
  (return false))

(fn GetBestInteractActor
  (return 0))

(fn GetBestHeavyInteractActor
  (return 0))

(fn ActivateAbility
  (return false))

(fn SetClientMovementPrediction
  (params (Enable :type Boolean)))

(fn IsOwningClient
  (return false))