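; Player character Blueprint for the visual layer: flashlight and proximity lights, mesh rotation, costumes, name tags, physics profiles and voice-driven speaking effects.
; Its events and functions are almost all stubs here, with empty bodies or default return values.
; Tick sub-events, server and multicast speaking-bubble events, and RepNotifies for death physics and costume outline the intended structure.
; Only the construction script and Mughost state update call their parents.
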(event Custom|BindGameplayEvent)

(event Custom|Tick_SpotLight)

(event Custom|Tick_SpeakingEffect)

(event Custom|ResetDeath)

(event Custom|SetPhysics
  (params (ProfileName :type Name)))

(event Custom|SpawnSpeakingBubbleEffect)

(event Custom|Server_CallSpawnSpeakingBubbleEffect)

(event Custom|Multicast_SpawnSpeakingBubbleFromServer)

(event Custom|Server_RegisterPlayerVoiceLevel
  (params (VoiceLevel :type Float%20%28double-precision%29)))

(event Custom|FlashLightLitVisual)

(event Custom|RefreshLightModule)

(event Custom|BindGameplayEventOnOwningClient)

(event Custom|Tick_Camera)

(event Custom|Force_MeshRotation)

(event Custom|FixCrashWhenSeamlessTravel)

(event Custom|TickPlayerNameRotation)

(event Custom|Force_ServerMeshRotation)

(event Custom|OnAudioEnvelopeValueChange
  (params (InputPin :type Float%20%28single-precision%29)))

(event Custom|Tick_MeshRotation)

(event Custom|Tick_ProximityLightPosition)

(event Custom|SetProximityLightFunctionMaterial)

(event Custom|Server_SendToServerMeshRotation
  (params (RelativeRotation :type Transform))
  (Variables|Default|SetRelative%20Rotation RelativeRotation))

(event Custom|Tick_LightPosition)

(event Custom|SetLightFunctionMaterial)

(event Custom|BindDeathEvent)

(event EventBeginPlay)

(event EventAfterCharacterReplicationRoleFound)

(event EventOnMughostStateUpdated
  (|CallParentFunction))

(event EventPlayerResetAudioCaptureComp)

(event EventTick
  (params (DeltaSeconds :type Float%20%28single-precision%29)))

(event EventPossessedonOwningClient)

(event EventPlayerSetPlayerNameVisibility
  (params (Visible :type Boolean) (Animated? :type Boolean)))

(event EventPlayerSetVisualforModule
  (params (Index :type Integer) (SKM_Ref :type Skeletal%20Mesh%20Object%20Reference)))

(event EventSetStationPhysics)

(event EventSetDefaultPhysics)

(event EventAfterCharacterReplicationRoleFoundonServer)

(event EventPlayerChangeShowPlayerNames
  (params (Yes :type Boolean)))

(event Custom|BindOtherEffects)

(event Custom|BindGameStateEffect_OwningClient)

(event Custom|BindGameStateEffect_OnServer)

(event Custom|BIndCostumeEffects)

(fn ConstructionScript
  (|CallParentFunction))

(fn PlayerCharInterfaceGetCameraOffset
  (return "0, 0, 0"))

(fn TogglePlayerFlashlight
  (params (FlashlightOn? :type Boolean)))

(fn OnRepSetDeathPhysicEnable)

(fn GetVoiceLevel
  (return 0.0))

(fn UpdateMeshforSpectatorMode)

(fn SetupEffects)

(fn PlayerGetVoiceVolume
  (return 0.0))

(fn GetSuspendedElementNiagara
  (return 0))

(fn CanRegisterVoiceLevel?
  (return false))

(fn GetTalkingEffectTreshold
  (return 0.0))

(fn SetupforTrailerVersion)

(fn GetLocalPlayer
  (return 0))

(fn GetLocalPlayerIsReady
  (return true))

(fn GetNewRelativeMeshTransform
  (return ""))

(fn OnRepCostumeRowName)

(fn AddorRemoveAgentNutSkm
  (params (Add :type Boolean)))

(fn UpdateFPSMeshScaleforWideScreens)

(fn GetCurrentCostumeRow
  (return ""))

(fn CheckPlayerNameVisibility)

(fn GetDynMaterialPlayerColor)

(fn PlayerHasVoiceGeneratedSounds?
  (return false))

(fn PlayerGetNormalizedVoiceVolume
  (return 0.0))

(fn PlayerGetSkinforCopyCat
  (return 0 "" "" 0 0))

(fn PlayerCharInterfaceGetInitMeshOffset
  (return "0, 0, 0"))

(fn GetTPSMeshAsset
  (return 0))

(fn GetTPSModulesMeshAsset
  (return 0 0))

(fn GetUCustomAudioCapture
  (return))