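; Player character Blueprint for a multiplayer game, declaring hooks for death and respawn, spectating, player color, voice chat and item hits such as crowbar, taser stick and EMP.
; Events are grouped into main, spectator, security and gameplay-effect graphs, alongside OnRep handlers and interface getters.
; Nearly every body is an empty stub or returns a default.
; Only owning-client possession and the construction script do anything, forwarding to the parent class.
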(event Custom|HandleCharacterMovementDeactivation)

(event Custom|HandleDeathEvent)

(event Custom|SetStationPhysics)

(event Custom|SetDefaultPhysics)

(event Custom|SetupPlayerStateIndex_Color)

(event Custom|BindMusicNearEnd)

(event Custom|UpdatePlayerColor)

(event Custom|HandleRespawnPlayer)

(event Custom|BeginPlay_SpawnAtLocation)

(event Custom|Client_HandleRespawnOnOwningClient)

(event Custom|AfterCharacterReplicationRoleFound_OnServer)

(event Custom|RefreshClosestPlayer)

(event Custom|HandleHealthLostEvent)

(event Custom|Client_HandleDeathEventOnOwningClient)

(event Custom|SetupPlayerStateIndex)

(event EventBeginPlay)

(event EventPlayerSetHudVisibility
  (params (NewVisibility :type Boolean)))

(event EventPossessedonOwningClient
  (|CallParentFunction))

(event EventEMPInteractionHitEvent
  (params (Player :type Actor%20Object%20Reference)))

(event EventPlayerResetAudioCaptureComp)

(event EventEnterSpectatorMode
  (params (CharacterToSpectate :type Character%20Object%20Reference)))

(event EventVOIPComponentRemoveAttenuationOverrides
  (params (Prio :type Float%20%28double-precision%29) (AttenuationAsset :type Sound%20Attenuation%20Object%20Reference)))

(event EventVOIPComponentAddAttenuationOverrides
  (params (AttenuationOverride :type Sound%20Attenuation%20Object%20Reference) (Priority :type Float%20%28double-precision%29)))

(event EventTick
  (params (DeltaSeconds :type Float%20%28single-precision%29)))

(event EventLoadPlayerGameplayChanger)

(event EventCrowbarInteractionHitEvent
  (params (Player :type Actor%20Object%20Reference)))

(event EventAfterCharacterReplicationRoleFound)

(event EventLeaveSpectatorMode)

(event EventPlayerSetVisualforModule
  (params (Index :type Integer) (SKM_Ref :type Skeletal%20Mesh%20Object%20Reference)))

(event EventTaserStickInteractionHitEvent
  (params (Player :type Actor%20Object%20Reference)))

(event EventPlayerReadyEventOnlyonServer)

(event Custom|Effects_AnimateTargetArmLength)

(event Custom|TriggerSpectatedPlayerChangeAfterDelay)

(event EventPlayerSetDelayBeforeEnteringSpectator
  (params (NewValue :type Float%20%28double-precision%29)))

(event Custom|Security_FixZipMeshIssue)

(event Custom|BindGameplayEvent_SecurityGraph_AllRoles)

(event Custom|BindGameplayEffectEventOnServer)

(event Custom|Multicast_SendVirusEvent)

(event EventLightSetLightOwner
  (params (Actor :type Actor%20Object%20Reference)))

(event EventLightToggleVisiblity
  (params (Visible :type Boolean)))

(fn ConstructionScript
  (|CallParentFunction))

(fn OnRepColor)

(fn IsNotInvincible
  (return true))

(fn TickSpectatorMode)

(fn OnRepCurrentSpectatorTransform)

(fn RefreshListPlayer
  (params (Tag :type Gameplay%20Tag%20Structure)))

(fn PlayerCharInterfaceGetClosestPlayerDistance
  (return 0.0))

(fn UpdateMeshforSpectatorMode)

(fn GetSpectatedPlayer
  (return 0))

(fn GetDynMaterialPlayerColor
  (return 0))

(fn GetOneShotEventInstigatorTags
  (params (InputPin :type Gameplay%20Event%20Data%20Structure))
  (return ""))

(fn HandleDeathReason
  (params (GameplayEventData :type Gameplay%20Event%20Data%20Structure%20%28by%20ref%29))
  (return))

(fn TickTimerEffects)

(fn PlayerIsUnderEMPEffect?
  (return false))

(fn PlayerGetLastDeathReason
  (return ""))

(fn GetSpectatorModeCameraSpeedFactor
  (return 0.0))

(fn PlayerCanUseImprovementStation
  (return false "0, 0, 0" 0))

(fn SetCharacterMeshAnimClass
  (params (NewClass :type Object%20Class%20Reference)))

(fn InitGCforServerOptionsModifier)

(fn GetTPSModulesMeshAsset
  (return 0 0))

(fn PlayerCharInterfaceGetInitMeshOffset
  (return "0, 0, 0"))

(fn PlayerCharInterfaceGetCameraOffset
  (return "0, 0, 0"))

(fn PlayerGetSkinforCopyCat
  (return 0 "" "" 0 0))

(fn PlayerGetNormalizedVoiceVolume
  (return 0.0))

(fn PlayerHasVoiceGeneratedSounds?
  (return false))