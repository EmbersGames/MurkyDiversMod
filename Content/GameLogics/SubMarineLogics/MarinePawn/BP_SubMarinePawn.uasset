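; Submarine pawn Blueprint with an interface for movement, depth, cannon hits and spawning surrounding islands and police, monster or neutral pawns.
; Most graphs are empty stubs, including movement, spawning and BeginPlayOnServer.
; The implemented speed boost holds full speed for its duration, then a timeline fades it out over a third of that time.
; Hostile selection favors police in depth zones tagged as police-controlled or influenced, and picks classes via shuffled index pools.
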(event Custom|RefreshSpawn)

(event Custom|SpawnTraderIsland)

(event Custom|SpawnIsland)

(event Custom|SetCurrentRudderRotate
  (params (Rudder1 :type Boolean) (NewValue :type Float%20%28double-precision%29)))

(event Custom|SpawnAltarIsland)

(event Custom|SetMaxSpeedByPlayersCount)

(event Custom|SpawnNewIslandOrSpecialIsland)

(event Custom|ProcessSpawnByDistanceReach)

(event Custom|InterpRotationToZero)

(event Custom|SpawnNeutralPawn)

(event Custom|SetInExploration)

(event Custom|CheckCloseToIsland)

(event Custom|Internal_BindGameStateEvent)

(event Custom|BeginPlayOnServer)

(event Custom|BindGameStateEvent)

(event Custom|PolicePawnHitMonsterPawn_Event
  (params (MonsterPawn :type Object%20Object%20Reference) (PolicePawn :type Object%20Object%20Reference) (Position :type Vector)))

(event EventBeginPlay
  (|CallParentFunction))

(event EventTick
  (params (DeltaSeconds :type Float%20%28single-precision%29))
  (|CallParentFunction DeltaSeconds))

(event Custom|BeginPlay_TreasureNet)

(event Custom|HitByTreasure
  (params (MarinePawn :type BP%20Marine%20Pawn%20Treasure%20Object%20Reference)))

(event Custom|Cannon_DestroyClosestPawn)

(event Custom|Multicast_PlayCannonMissEffect)

(event Custom|BoostSpeedOnServer
  (params (BoostDuration :type Float%20%28double-precision%29))
  (Variables|State|SetLocalBoostSpeed "0, 0, 0")
  (Variables|Boost|SetBoostDirection (Variables|Default|GetDirection))
  (Variables|Boost|SetBoostSpeed (Variables|Boost|GetMaxBoostSpeed))
  (Variables|Boost|SetBoostAcceleration (Variables|Boost|GetMaxBoostAcceleration))
  (Utilities|FlowControl|Delay BoostDuration)
  (Components|Timeline|SetPlayRate (Variables|Default|GetBoostOutLerp) (/ 1.0 (* BoostDuration 0.33)))
  (bind _lerp (Timeline|BoostOutLerp PlayFromStart)
    (:Update
      (Variables|Boost|SetBoostSpeed (Math|Float|Lerp 0.0 (Variables|Boost|GetMaxBoostSpeed) _lerp)))))

(event Custom|BoostSpeed_Effect)

(event Custom|BindDepthEvents_ServerOnly)

(event Custom|ChangeDepth)

(fn ConstructionScript
  (|CallParentFunction))

(fn OnRepIsland)

(fn GetPositionClosetoPlayerOutOfSonar
  (return "0, 0, 0"))

(fn GetDirectiontoCrossPlayer
  (params (LocalPosition :type Vector))
  (return "0, 0, 0"))

(fn SpawnHostilePawn
  (params (IsPolice :type Boolean)))

(fn GetPawninDistance
  (params (Distance :type Float%20%28double-precision%29))
  (return 0))

(fn GetPoliceCount
  (params (Pawns :type Array%20of%20BP%20Marine%20Pawn%20Base%20Object%20References))
  (return 0))

(fn GetNeutralCount
  (params (Pawns :type Array%20of%20BP%20Marine%20Pawn%20Base%20Object%20References))
  (return 0))

(fn GetMonsterCount
  (params (Pawns :type Array%20of%20BP%20Marine%20Pawn%20Base%20Object%20References))
  (return 0))

(fn SetinNavigationMode
  (params (State :type Boolean)))

(fn HitbyMarinePawn
  (params (Pawn :type BP%20Marine%20Pawn%20Base%20Object%20Reference)))

(fn GetPositionClosetoPlayerOutOfSonarforIsland
  (return "0, 0, 0"))

(fn OnRepPawns)

(fn SetupNameList)

(fn DestroyPawnandIslandTooFar)

(fn AddValidName
  (params (Name :type Name%20%28by%20ref%29)))

(fn GetUniqueName
  (return "None"))

(fn RefreshNarrowBandList)

(fn IsArrayDifferent
  (params (Arr1 :type Array%20of%20Strings) (Arr2 :type Array%20of%20Strings))
  (return false))

(fn GetTreasureNet
  (return))

(fn GetRotateSpeed
  (return 0.0))

(fn HasRudderSpeedImprovement
  (return false))

(fn GetClosestPawn
  (return 0))

(fn PerformMovement)

(fn GetSpawnSettingsforCurrentDepthLayer
  (return))

(fn ShouldSpawnSpecialIsland
  (return false))

(fn GetTreasureorNeutralMarinePawnClass
  (return 0))

(fn GetHostilePawnClass
  (params (Police :type Boolean))
  (Utilities|FlowControl|Sequence
    (:then_1
      (Utilities|Array|Shuffle (LocalVariables|GetMonsterPoolIndex))
      (Utilities|Array|Shuffle (LocalVariables|GetPolicePoolIndex))
      (return (select Police (Utilities|Select :Index (Utilities|Array|Get(acopy) (LocalVariables|GetPolicePoolIndex)) :Option%200 0 :Option%201 0 :Option%202 0) (Utilities|Select :Index (Utilities|Array|Get(acopy) (LocalVariables|GetMonsterPoolIndex)) :Option%200 0 :Option%201 0 :Option%202 0))))))

(fn GetMaxSpeedWithoutModifier
  (return 0.0))

(fn GetMinDistanceforMonster
  (return 0.0))

(fn GameStateHaveTag?
  (params (GameplayTag :type Gameplay%20Tag%20Structure))
  (return false))

(fn GetGameStateDepthComp
  (return 0))

(fn HostileIsPoliceorMonsterNewSpawn
  (Utilities|FlowControl|Sequence
    (:then_0
      (if (Utilities|GameStateHaveTag? "(TagName=\"Submarine.State.Depth.IsInPoliceControlledZone\")")
        (return (<= (Math|Random|RandomFloat) 0.875))))
    (:then_1
      (if (Utilities|GameStateHaveTag? "(TagName=\"Submarine.State.Depth.IsInPoliceInfluenceZone\")")
        (return (<= (Math|Random|RandomFloat) 0.75))))
    (:then_2
      (return (Math|Random|RandomBool)))))

(fn GetMaxPoliceSubMarinePawn
  (return 10))

(fn GetMaxMonsterforPoliceRange
  (return 20))

(fn GetMinDistancetoSpawnIsland
  (return 0.0 0.0))

(fn GetInitialDistanceforLastIslandReach
  (return 4e+02))

(fn SpecialExpedBadluckProtection
  (params (RandomBool :type Boolean))
  (return false))

(fn GetMinDistanceforPolice
  (return 0.0))

(fn GetIncrChancetoSpawnSpecialIsland
  (return 0.0))

(fn CanSpawnMonster
  (return false))

(fn CanSpawnPolice
  (return false))

(fn GetMaxMonsterMarinePawn
  (return 0))

(fn SpawnIslandforChallenge)