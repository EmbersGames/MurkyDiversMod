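; BP_SonarIsland_Special is a special sonar island variant in the submarine game logic, configured by overriding getter functions.
; It supplies a fixed directional light rotation, pale green-tinted color and intensity.
; It disables the spawn system, skips nav rebuilds and reports false for the 2, 4 and 8-player sub checks.
; The sequence and smooth cube material functions are empty, and construction only calls the parent script.
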(fn ConstructionScript
  (|CallParentFunction))

(fn GetStartSequence
  (return 0))

(fn GetEndSequence
  (return 0))

(fn GetLoopSequence
  (return 0))

(fn GetSmoothCubeMaterial
  (return 0))

(fn GetDirectionalLightRotation
  (return "540.000000,540.000000,-39.850000"))

(fn IsNeededtoRebuildNav?
  (return false))

(fn LoadSequence
  (params (Sequence :type Level%20Sequence%20Soft%20Object%20Reference))
  (return 0))

(fn IsSub2Players?
  (return false))

(fn IsSub4Players?
  (return false))

(fn IsSub8Players?
  (return false))

(fn GetDirectionalLightColor
  (return "(R=0.807843,G=1.000000,B=0.929412,A=1.000000)"))

(fn GetDirectionalLightIntensity
  (return 3.0))

(fn DisableSpawnSystem?
  (return true))