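; BP_MarinePawn_Base is the base submarine pawn, declaring a shared interface for movement, rotation and fade-off.
; Movement, goal setters, fade events and the fade RepNotify are empty stubs, presumably for child Blueprints to override.
; Getters expose rotate speed, max speed and max acceleration variables, while delta-seconds factor and unmodified max speed return placeholder constants.
; BeginPlay only calls its parent.
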(event Custom|StartFadeOff_Client)

(event Custom|SetStartFade_OnlyServer)

(event EventBeginPlay
  (|CallParentFunction))

(event EventTick
  (params (DeltaSeconds :type Float%20%28single-precision%29)))

(fn ConstructionScript)

(fn PerformRotation)

(fn PerformMovement)

(fn SetRotationGoal
  (params (NewValue :type Float%20%28double-precision%29)))

(fn SetSpeedGoal
  (params (NewValue :type Float%20%28double-precision%29)))

(fn SetDirection
  (params (NewValue :type Vector)))

(fn SetSpeed
  (params (NewValue :type Vector)))

(fn GetRotateSpeed
  (return (Variables|Movement|GetRotateSpeed)))

(fn UpdateIsMoving)

(fn GetSpeedMax
  (return (Variables|Movement|GetSpeedMax)))

(fn GetAccelerationMax
  (return (Variables|Movement|GetAccelerationMax)))

(fn GetDeltaSecondsFactor
  (return 1.0))

(fn GetMaxSpeedWithoutModifier
  (return 0.0))

(fn OnRepFadeOff)