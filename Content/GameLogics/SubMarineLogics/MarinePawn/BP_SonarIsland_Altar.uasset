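; Altar variant of a sonar island Blueprint in the submarine logic, configuring the look of that level through overrides of parent functions.
; It supplies the Altar volumetric level material for the smooth cube, plus a fixed rotation, pale blue-violet color and intensity for the directional light.
; It adds no runtime logic of its own, as the construction script defers to the parent and the event graph stubs are disabled.
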(event EventBeginPlay
  (|CallParentFunction) ; This node is disabled and will not be called.\nDrag off pins to build functionality.
)

(event Collision|EventActorBeginOverlap
  (params (OtherActor :type Actor%20Object%20Reference)))

(event EventTick
  (params (DeltaSeconds :type Float%20%28single-precision%29)))

(fn ConstructionScript
  (|CallParentFunction))

(fn GetSmoothCubeMaterial
  (return "/Game/Effects/Volumetric/M_Volumetric_Level_Altar.M_Volumetric_Level_Altar"))

(fn GetDirectionalLightRotation
  (return "90.000000,0.000000,0.000000"))

(fn GetDirectionalLightColor
  (return "(R=0.481432,G=0.444894,B=0.967014,A=1.000000)"))

(fn GetDirectionalLightIntensity
  (return 13.0))