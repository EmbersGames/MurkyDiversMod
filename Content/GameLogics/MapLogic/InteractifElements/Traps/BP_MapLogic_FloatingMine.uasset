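; BP_MapLogic_FloatingMine is a floating mine map trap with events for trigger overlap, EMP and taser-stick hits, and chaining from other mines.
; Replicated state drives clients: OnRep_StartExplode starts countdown effects, and OnRep_IsDestroyed plays explosion effects, then hides the actor and disables collision.
; Damage factor is full within DeathDistanceToMine, falling linearly to a quarter at the ExplosionZone radius.
; The event bodies, construction script and OnRep_SpawnFX are empty here.
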(event OnComponentBeginOverlap(Trigger)
  (params (OverlappedComponent :type Primitive%20Component%20Object%20Reference) (OtherActor :type Actor%20Object%20Reference) (OtherComp :type Primitive%20Component%20Object%20Reference) (OtherBodyIndex :type Integer) (bFromSweep :type Boolean) (SweepResult :type Hit%20Result%20Structure%20%28by%20ref%29)))

(event Custom|DestroyEvent)

(event Custom|Explode_EffectsEvent)

(event Custom|StartCountdown_EffectsEvent)

(event Custom|ExplodeByAnotherMine)

(event EventTaserStickInteractionHitEvent
  (params (Player :type Actor%20Object%20Reference)))

(event EventEMPInteractionHitEvent
  (params (Player :type Actor%20Object%20Reference)))

(fn ConstructionScript)

(fn OnRepIsDestroyed
  (CallFunction|ExplodeEffectsEvent)
  (Collision|SetActorEnableCollision false)
  (Rendering|SetActorHiddenInGame true))

(fn OnRepStartExplode
  (CallFunction|StartCountdownEffectsEvent))

(fn OnRepSpawnFX)

(fn GetDamageFactorforDistance
  (params (CurrentActor :type Actor%20Object%20Reference))
  (bind _returnvalue (Transformation|GetActorLocation CurrentActor))
  (bind _explosionzone (Variables|Default|GetExplosionZone))
  (bind _returnvalue_2 (Transformation|GetWorldLocation _explosionzone))
  (bind _returnvalue_3 (Math|Vector|Distance(Vector) _returnvalue _returnvalue_2))
  (return (Math|Float|Lerp 0.25 1.0 (Math|Float|SelectFloat 1.0 (Math|Float|Lerp 1.0 0.0 (Math|Float|Clamp(Float) (/ (- _returnvalue_3 (Variables|Default|GetDeathDistanceToMine)) (- (Components|Sphere|GetScaledSphereRadius (Variables|Default|GetExplosionZone)) (Variables|Default|GetDeathDistanceToMine))))) (<= _returnvalue_3 (Variables|Default|GetDeathDistanceToMine))))))