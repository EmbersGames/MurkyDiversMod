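; Base item for map-logic objects, deriving from a parent item class and presenting itself as a grabbable, non-heavy, belt-storable, non-tool actor.
; Most inherited physics, attachment, cart, user and replication handlers are overridden empty, while lifecycle, player tagging and some interaction and collision events forward to the parent.
; Interaction queries mostly return fixed defaults, with the grab offset read from the mesh's GrabItem_Socket.
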(event Custom|UserChange)

(event Custom|RefreshCollisionAndPhysic
  (params (Data :type Struct%20Attachment%20Data%20Structure)))

(event Custom|Multicast_ForceRefreshRelativeTransform
  (params (Transform :type Transform)))

(event Custom|RefreshPhysicMeshCollisionEnabled)

(event Custom|RefreshPhysicEnableOnServer)

(event Custom|AddRotationToObject)

(event Custom|SetIsInCooldown
  (params (Cooldown :type Boolean)))

(event Custom|OnComponentSleep_Event
  (params (SleepingComponent :type Primitive%20Component%20Object%20Reference) (BoneName :type Name)))

(event Custom|OnComponentWake_Event
  (params (WakingComponent :type Primitive%20Component%20Object%20Reference) (BoneName :type Name)))

(event EventBeginPlay
  (|CallParentFunction))

(event EventDestroyed
  (|CallParentFunction))

(event EventRefreshActorCollisionEnabled
  (|CallParentFunction))

(event EventItemSetAttachDataClientPrediction
  (params (Data :type Struct%20Attachment%20Data%20Structure)))

(event EventItemUseItemEvent
  (params (GAS :type Ability%20System%20Component%20Object%20Reference)))

(event EventItemSetUser
  (params (User :type Actor%20Object%20Reference)))

(event EventItemAddForcetoItem
  (params (Forward :type Vector :default "0, 0, 0") (Power :type Float%20%28double-precision%29)))

(event EventEndPlay
  (params (EndPlayReason :type EEndPlayReason%20Enum :default "Destroyed"))
  (|CallParentFunction EndPlayReason))

(event EventItemShredEvent
  (params (WasInCart :type Actor%20Object%20Reference)))

(event EventItemSetinPredicationAttachmentState
  (params (State :type Boolean)))

(event EventInteractInteractionEvent
  (|CallParentFunction))

(event EventItemSetIsinCart
  (params (Yes :type Boolean) (Cart :type Actor%20Object%20Reference)))

(event EventItemSetAttachData
  (params (Data :type Struct%20Attachment%20Data%20Structure)))

(event EventInteractSetActorCollisionEnable
  (params (Enable :type Boolean))
  (|CallParentFunction Enable))

(event EventItemSetRelativeTransformbyServer
  (params (Transform :type Transform)))

(event EventItemSpawninDispenser
  (params (Forward :type Vector :default "0, 0, 0") (Power :type Float%20%28double-precision%29) (Origin :type Vector :default "0, 0, 0")))

(event EventInteractRefreshPhysicEnable
  (|CallParentFunction))

(fn ConstructionScript
  (|CallParentFunction))

(fn InteractCanInteract?
  (return false))

(fn InteractIsGrabableActor?
  (return true))

(fn InteractIsSimpleInteract?
  (return false))

(fn OnRepIsinCart)

(fn CastRule
  (params (Rule :type Enum_AttachmentRule%20Enum :default "NewEnumerator0"))
  (return "KeepRelative"))

(fn OnRepNewScale3D)

(fn RefreshAttachData
  (params (AttachmentData :type Struct%20Attachment%20Data%20Structure%20%28by%20ref%29) (IsServerData :type Boolean)))

(fn AddTagtoPlayer
  (params (ActualPlayer :type Actor%20Object%20Reference))
  (|CallParentFunction ActualPlayer))

(fn OnRepServerDataAttach)

(fn RemoveTagtoPlayer
  (params (ActualPlayer :type Actor%20Object%20Reference))
  (|CallParentFunction ActualPlayer))

(fn RefreshRecentPlayerorInteraction)

(fn InteractGetGrabOffSet
  (return (Transformation|GetSocketTransform (Variables|Default|GetStaticMeshComponent) "GrabItem_Socket" "RTS_Component")))

(fn OnRepUser)

(fn OnRepDisableInteraction)

(fn InteractGetInteractionAnchorWorldLocation
  (return "0, 0, 0"))

(fn InteractIsStationGrabable?
  (return false))

(fn InteractIsHeavyGrabableActor?
  (return false))

(fn ItemCanbeGrapplingAttract?
  (return (Variables|Default|GetCanBeGrapplingAttract)))

(fn ItemCanPutinBelt
  (return true))

(fn ItemCartValue
  (return 0))

(fn ItemGetAttachData
  (return (Variables|attach|GetServerData_Attach)))

(fn ItemGetAttachDataClientPrediction
  (return ""))

(fn ItemGetGrabSound
  (return 0))

(fn ItemGetImageinBelt
  (return 0 "None"))

(fn ItemGetMontagetoPlay
  (return 0))

(fn ItemGetOldUser
  (return 0))

(fn ItemGetPlayerOwnerAttach
  (return 0))

(fn ItemGetUser
  (return (Variables|User|GetUser)))

(fn ItemIsinCart?
  (return false 0))

(fn ItemIsTool
  (return false))

(fn ItemUseGetAbilitytoActivate
  (return ""))