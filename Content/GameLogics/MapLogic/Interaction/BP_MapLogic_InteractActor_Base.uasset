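; Base Blueprint for interactable map-logic actors, answering interaction queries with defaults: interactable and grabbable, but not heavy, simple or station-grabbable.
; Scene components supply the grab offset and interaction anchor.
; Helper functions register or remove the actor in the player's Ability System Component under an items-in-range gameplay tag.
; A RepNotify calls the collision refresh event, which is empty here, as are the sphere overlap handlers.
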(event OnComponentBeginOverlap(Sphere)
  (params (OverlappedComponent :type Primitive%20Component%20Object%20Reference) (OtherActor :type Actor%20Object%20Reference) (OtherComp :type Primitive%20Component%20Object%20Reference) (OtherBodyIndex :type Integer) (bFromSweep :type Boolean) (SweepResult :type Hit%20Result%20Structure%20%28by%20ref%29)))

(event OnComponentEndOverlap(Sphere)
  (params (OverlappedComponent :type Primitive%20Component%20Object%20Reference) (OtherActor :type Actor%20Object%20Reference) (OtherComp :type Primitive%20Component%20Object%20Reference) (OtherBodyIndex :type Integer)))

(event Custom|InitOverlaps)

(event Custom|RefreshActorCollisionEnabled)

(event Custom|BindGameStateEvent)

(event EventBeginPlay
  (|CallParentFunction))

(event EventInteractSetActorCollisionEnable
  (params (Enable :type Boolean)))

(fn ConstructionScript)

(fn AddTagtoPlayer
  (params (ActualPlayer :type Actor%20Object%20Reference))
  (if (not (Utilities|Array|ContainsItem (Class|AbilitySystemComponentBase|GetObjectsStoredwithGameplayTag (Class|AbilitySystemComponentBase|GetAbilitySystemComp ActualPlayer) "(TagName=\"Player.State.Interact.ItemInRange_Objects\")") self))
    (Class|AbilitySystemComponentBase|AddObjectStoredwithGameplayTag (Class|AbilitySystemComponentBase|GetAbilitySystemComp ActualPlayer) "(TagName=\"Player.State.Interact.ItemInRange_Objects\")" self)))

(fn RemoveTagtoPlayer
  (params (ActualPlayer :type Actor%20Object%20Reference))
  (Class|AbilitySystemComponentBase|RemoveObjectStoredwithGameplayTag (Class|AbilitySystemComponentBase|GetAbilitySystemComp ActualPlayer) "(TagName=\"Player.State.Interact.ItemInRange_Objects\")" self))

(fn OnRepActorCollisionEnable
  (CallFunction|RefreshActorCollisionEnabled))

(fn InteractCanInteract?
  (return true))

(fn InteractGetGrabOffSet
  (return (Transformation|GetRelativeTransform (Variables|Default|GetPlayerGrabPos))))

(fn InteractGetInteractionAnchorWorldLocation
  (return (Transformation|GetWorldLocation (Variables|Default|GetInteractPosition))))

(fn InteractIsGrabableActor?
  (return true))

(fn InteractIsHeavyGrabableActor?
  (return false))

(fn InteractIsSimpleInteract?
  (return false))

(fn InteractIsStationGrabable?
  (return false))