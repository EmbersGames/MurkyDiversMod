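; BP_ServerGameOptions_Comp is a component that holds server game options, exposing typed getters for current and default values.
; SetGamesOptionsFromMap clears and refills parallel name and value arrays from a map.
; The getters, preset loading and apply routines, including the station upgrade, show only empty bodies or constant returns here.
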(event EventBeginPlay
  (|CallParentFunction))

(event Custom|ApplyGameOptions)

(event Custom|ApplyGameOptions_DependingOnGameStateGasComp)

(fn InternalGetGameOptionValue
  (params (Option :type Data%20Table%20Row%20Handle%20Structure))
  (return ""))

(fn GetGameOptionValueasBool
  (params (Option :type Data%20Table%20Row%20Handle%20Structure))
  (return false false))

(fn GetGameOptionValueasFloat
  (params (Option :type Data%20Table%20Row%20Handle%20Structure))
  (return false 0.0))

(fn GetGameOptionValueasTagList
  (params (Option :type Data%20Table%20Row%20Handle%20Structure))
  (return true 0))

(fn GetGameOptionValueasFloatArray
  (params (Option :type Data%20Table%20Row%20Handle%20Structure))
  (return true 0))

(fn LoadGameOptionfromPreset
  (params (PresetDatatable :type Data%20Table%20Object%20Reference)))

(fn SetGamesOptionsfromMap
  (params (Options :type Map%20of%20Names%20to%20Structs))
  (Utilities|Array|Clear (Variables|Default|GetGameOptionValues))
  (Utilities|Array|Clear (Variables|Default|GetGameOptionNames))
  (bind _keys (Utilities|Map|Keys Options))
  (for _array_element _keys
    (Utilities|Array|Add (Variables|Default|GetGameOptionNames) _array_element)
    (Utilities|Array|Add (Variables|Default|GetGameOptionValues) (.Value (Utilities|Map|Find Options _array_element)))))

(fn GetAllGameOptionasMap
  (return 0 "None"))

(fn GetDefaultGameOptionValueasBool
  (params (Option :type Data%20Table%20Row%20Handle%20Structure))
  (return false false))

(fn GetDefaultGameOptionValueasFloat
  (params (Option :type Data%20Table%20Row%20Handle%20Structure))
  (return false 0.0))

(fn GetDefaultGameOptionValueasTagList
  (params (Option :type Data%20Table%20Row%20Handle%20Structure))
  (return false 0))

(fn GetDefaultGameOptionValueasFloatArray
  (params (Option :type Data%20Table%20Row%20Handle%20Structure))
  (return false 0))

(fn GetDefaultGameOptionValue
  (params (Option :type Data%20Table%20Row%20Handle%20Structure))
  (return ""))

(fn ApplyGameOptionsUpgradeAllStations)

(fn GetGameOptionValue
  (params (Option :type Data%20Table%20Row%20Handle%20Structure))
  (return (Utilities|Struct|MakeStruct_GameOptionValue true 0 0)))