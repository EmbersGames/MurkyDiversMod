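; GameState component for the submarine depth system, covering current depth, biome and level selection, and police progression.
; Nearly every function and event is an empty stub or returns a default, including biome choice, bad-luck security and server option filtering.
; The live logic counts down expeditions before setting the depth-activation gameplay tag on the GameState's ability system.
; The CurrentDepth OnRep sends a gameplay event to the GameState to update the depth display.
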(event Custom|ImproveDepth
  (params (Index :type Integer)))

(event Custom|PoliceProgression)

(event Custom|UpdatePoliceTags)

(event Custom|Multicast_PlayImproveDepth_Effect)

(event Custom|UpdateAnalytics)

(event Custom|CloseGateTuto)

(event EventBeginPlay)

(fn GetCurrentBiomeRowName
  (return "None"))

(fn GetCurrentDepth
  (return (Variables|Default|GetCurrentDepth)))

(fn GetCurrentBiomeLevel
  (return 0))

(fn GetGameState
  (return))

(fn GetStarScore
  (return 0.0))

(fn GetCurrentSpawnDataTablebyBiome
  (return 0))

(fn GetPoliceProgressionSpeed
  (return 0.0))

(fn SelectNextBiomeRows
  (return 0))

(fn SelectRowwithSpawnRateValue
  (params (BiomeSpawnRate :type Map%20of%20Names%20to%20Reals) (SpawnRateValue :type Float%20%28double-precision%29))
  (return "None"))

(fn SelectNextBiomesManager
  (return 0))

(fn SelectNextBiomeLevels
  (params (Array :type Array%20of%20Names))
  (return 0))

(fn GetBiomeChoiceDatas
  (return 0))

(fn OnRepBiomeChoiceDatas)

(fn OnRepCurrentPoliceDepth)

(fn GetPoliceInfluenceDistance
  (return (Variables|Police|GetPoliceInfluenceDistance)))

(fn GetPoliceCurrentDepth
  (return (Variables|Police|GetCurrentPoliceDepth)))

(fn OnRepCurrentDepth
  (Ability|SendGameplayEventtoActor (Game|GetGameState) "(TagName=\"Submarine.State.Depth.UpdateDisplayCurrentDepth_Event\")"))

(fn GetBiomeLevelwithRate
  (params (CurrentBiome :type Boolean))
  (return 0))

(fn CheckCanChooseBiome
  (return false))

(fn CheckCanActivateDepthSystem
  (if (not (Class|AbilitySystemComponentBase|HasGameplayTag (Class|AbilitySystemComponentBase|GetAbilitySystemComp (Game|GetGameState)) "(TagName=\"Submarine.State.Depth.IsActivate\")"))
    (Variables|Default|SetCurrentExpedNumberToActivateDepthSystem (- (Variables|Default|GetCurrentExpedNumberToActivateDepthSystem) 1))
    (if (<= (Variables|Default|GetCurrentExpedNumberToActivateDepthSystem) 0)
      (Class|AbilitySystemComponentBase|SetGameplayTagCount (Class|AbilitySystemComponentBase|GetAbilitySystemComp (Game|GetGameState)) "(TagName=\"Submarine.State.Depth.IsActivate\")" 1))))

(fn OnRepCurrentBiomeLevel)

(fn OnRepCurrentBiomeRowName)

(fn CheckHaveNextLevelBiome
  (params (Levels :type Array%20of%20Integers))
  (return true))

(fn NextLevelBadLuckSecurity
  (params (Levels :type Array%20of%20Integers) (BiomesRow :type Array%20of%20Names))
  (return 0 0))

(fn GetSelectNextBiomeLevelCurrentValue
  (return 0))

(fn InitNewGame)

(fn FilterAvailableBiomes
  (params (Biomes :type Array%20of%20Names))
  (return 0))

(fn HasPoliceProgressionOption
  (return false))

(fn CheckifBiomeIsAvalaibleinServerOptions
  (params (BIomeTag :type Gameplay%20Tag%20Structure))
  (return false))

(fn GetLevelsAvailableListServerOptions)

(fn CheckandReturnAvailableLevel
  (params (Level :type Integer) (UpperPriority :type Boolean))
  (return 0))

(fn CheckandReturnBiomeSecurity)

(fn GetCurrentSpawnWeightwithLabSecurity
  (params (Row :type Name))
  (return 0.5))

(fn BiomeBadLuckSecurity
  (params (BiomeRows :type Array%20of%20Names))
  (return 0))

(fn DefineNewRandomStream
  (params (DungeonSeed :type Integer)))